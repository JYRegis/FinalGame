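; PC_PLAY is the gameplay player controller that handles backpack input.
; BeginPlay registers the Enhanced Input mapping context, and the OpenBP action toggles the HUD's backpack widget.
; FUNOPENBp switches widget visibility, input mode and mouse cursor together.
; Keys 1 and 2 call a PlayerState event to add items by ID, which its name marks as server-side.
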(event `self.ReceiveBeginPlay`
  (bind _returnvalue (pcsubsystem `EnhancedInputLocalPlayerSubsystem` self))
  (`/Engine/EditorBlueprintResources/StandardMacros.IsValid` _returnvalue
    (:`Is Valid`
      (`EnhancedInputSubsystemInterface.AddMappingContext` _returnvalue "/Game/增强输入/Mapping_input.Mapping_input" 0 (struct)))))

(event `InputAction|OpenBP`
  (params (Key :type "Key Structure"))
  ;[0 0.15 0.04166 0.5] 按F打开背包
  (:`Pressed`
    (`self.FUN_OPENBp` (not (`Widget.IsVisible` (`/Game/蓝图/Hud_play.umg_bp` (`/Game/蓝图/Funl_play.FUNL_GetHUD`)))))))

(event `Key|One`
  (params (Key :type "Key Structure"))
  ;[0.15 0 0.01974 0.5] 添加物品按键
  (:`Pressed`
    (`/Game/蓝图/PS_PLAY.EVE_Server_Add_Rs_ByID` (`/Game/蓝图/Funl_play.FUNL_GetPlayerState`) "1")))

(event `Key|Two`
  (params (Key :type "Key Structure"))
  ;[0.15 0 0.01974 0.5] 添加物品按键
  (:`Pressed`
    (`/Game/蓝图/PS_PLAY.EVE_Server_Add_Rs_ByID` (`/Game/蓝图/Funl_play.FUNL_GetPlayerState`) "2")))

(fn `FUN_OPENBp`
  (params (Open :type Boolean))
  (bind _umg_bp (`/Game/蓝图/Hud_play.umg_bp` (`/Game/蓝图/Funl_play.FUNL_GetHUD`)))
  (if Open
    (`Widget.SetVisibility` _umg_bp "SelfHitTestInvisible")
    (`WidgetBlueprintLibrary.SetInputMode_GameAndUIEx` self _umg_bp)
    (set `self.bShowMouseCursor` true)
    (else
      (`Widget.SetVisibility` (`/Game/蓝图/Hud_play.umg_bp` (`/Game/蓝图/Funl_play.FUNL_GetHUD`)) "Collapsed")
      (`WidgetBlueprintLibrary.SetInputMode_GameOnly` self)
      (set `self.bShowMouseCursor` false))))

(fn `UserConstructionScript`)